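; Player controller for the Infidel FPS that owns the local player's HUD widget.
; On BeginPlay, for the local controller only, it creates the HUD, adds it to the viewport and seeds it with the possessed FPSCharacter's health and, if a valid weapon exists, its ammo.
; UpdateHUDHealth and UpdateHUDAmmo pass later value changes through to the widget.
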(event EventBeginPlay
  (bind _self self)
  (if (Pawn|IsLocalPlayerController _self)
    (bind _returnvalue (UserInterface|CreateWidget "/Game/Infidel/Blueprints/HUD/HUD.HUD_C" _self))
    (bind _output_get (Variables|Default|SetHUD _returnvalue))
    (UserInterface|Viewport|AddtoViewport _output_get 0)
    (bind _asfpscharacter (Utilities|Casting|CastToFPSCharacter (Pawn|GetControlledPawn)))
    (Default|UpdateHealth (Variables|Default|GetHUD) (Variables|/Game/Infidel/Blueprints/FPSCharacter.FPSCharacter_C|GetHealth _asfpscharacter))
    (Utilities|IsValid (Variables|/Game/Infidel/Blueprints/FPSCharacter.FPSCharacter_C|GetWeapon _asfpscharacter)
      (:Is%20Valid
        (Default|UpdateAmmo (Variables|Default|GetHUD) (Variables|/Game/Infidel/Blueprints/WeaponBase.WeaponBase_C|GetAmmo (Variables|/Game/Infidel/Blueprints/FPSCharacter.FPSCharacter_C|GetWeapon _asfpscharacter)))))))

(event EventTick
  (params (DeltaSeconds :type Float%20%28single-precision%29)))

(fn ConstructionScript)

(fn UpdateHUDHealth
  (params (Health :type Float%20%28single-precision%29))
  (Default|UpdateHealth (Variables|Default|GetHUD) Health))

(fn UpdateHUDAmmo
  (params (Ammo :type Integer))
  (Default|UpdateAmmo (Variables|Default|GetHUD) Ammo))