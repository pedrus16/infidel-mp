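; Game mode for a traitor-versus-innocents match, handling match start, role assignment and win conditions.
; Once enough players log in, it destroys the session, sets the game state's end time and randomly assigns traitors.
; Pickup slot events trigger an innocent win when all slots are filled.
; A separate death check counts living players per side and reports the winner to the game state.
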(event Custom|OnItemPlaced
  (CallFunction|CheckVictoryObjectiveComplete))

(event EventBeginPlay
  (bind _outactors (Actor|GetAllActorsOfClass "/Game/Infidel/Blueprints/BP_PickupSlot.BP_PickupSlot_C"))
  (bind _output_get (Variables|Game|SetItemSlots _outactors))
  (for _array_element _output_get
    (EventDispatchers|BindEventtoItemPlaced _array_element (delegate Custom|OnItemPlaced))))

(event EventTick
  (params (DeltaSeconds :type Float%20%28single-precision%29)))

(event EventPostLogin
  (params (NewPlayer :type Player%20Controller%20Object%20Reference))
  (bind _returnvalue (Class|GameModeBase|GetNumPlayers))
  (if (>= _returnvalue (Variables|Game|GetPlayerCount))
    (|DestroySession (Game|GetPlayerController 0)
      (:OnSuccess
        (CallFunction|StartGame)))))

(fn ConstructionScript)

(fn StartGame
  (bind _asdefault_game_state (Utilities|Casting|CastToDefaultGameState (Game|GetGameState)))
  (Variables|/Game/Infidel/Blueprints/DefaultGameState.DefaultGameState_C|SetEndTimeSeconds _asdefault_game_state (+ (GameState|GetServerWorldTimeSeconds _asdefault_game_state) (Variables|Game|GetGameDurationSecond)))
  ;[1 1 1] Assign roles
  (Utilities|Array|Shuffle (Variables|/Script/Engine.GameStateBase|GetPlayerArray _asdefault_game_state))
  (for (_array_element _array_index) (Variables|/Script/Engine.GameStateBase|GetPlayerArray _asdefault_game_state)
    (bind _asdefault_player_state (Utilities|Casting|CastToDefaultPlayerState _array_element))
    (Variables|/Game/Infidel/Blueprints/DefaultPlayerState.DefaultPlayerState_C|SetIsTraitor _asdefault_player_state (< _array_index (Variables|Game|GetTraitorCount)))))

(fn CheckVictoryObjectiveComplete
  (bind _itemslots (Variables|Game|GetItemSlots))
  (LocalVariables|SetItemSlotCompleted 0)
  (for _array_element _itemslots
    (Utilities|IsValid (Variables|/Game/Infidel/Blueprints/BP_PickupSlot.BP_PickupSlot_C|GetItem _array_element)
      (:Is%20Valid
        (Math|Integer|IncrementInt (LocalVariables|GetItemSlotCompleted)))))
  (if (== (LocalVariables|GetItemSlotCompleted) (Utilities|Array|Length _itemslots))
    (bind _asdefault_game_state (Utilities|Casting|CastToDefaultGameState (Game|GetGameState)))
    (Default|GameEnded _asdefault_game_state false)))

(fn CheckVictoryPlayerDied
  (bind _returnvalue (Game|GetGameState))
  (LocalVariables|SetAliveTraitorCount 0)
  (LocalVariables|SetAliveInnocentCount 0)
  (bind _outactors (Actor|GetAllActorsOfClass "/Game/Infidel/Blueprints/FPSCharacter.FPSCharacter_C"))
  (for _array_element _outactors
    (bind _asdefault_player_state (Utilities|Casting|CastToDefaultPlayerState (Variables|/Script/Engine.Pawn|GetPlayerState _array_element)))
    (if (not (Variables|/Game/Infidel/Blueprints/FPSCharacter.FPSCharacter_C|GetDead _array_element))
      (if (Variables|/Game/Infidel/Blueprints/DefaultPlayerState.DefaultPlayerState_C|GetIsTraitor _asdefault_player_state)
        (Math|Integer|IncrementInt (LocalVariables|GetAliveTraitorCount))
        (else
          (Math|Integer|IncrementInt (LocalVariables|GetAliveInnocentCount))))))
  (if (<= (LocalVariables|GetAliveInnocentCount) 0)
    (bind _asdefault_game_state (Utilities|Casting|CastToDefaultGameState _returnvalue))
    (Default|GameEnded _asdefault_game_state true)
    (elif (<= (LocalVariables|GetAliveTraitorCount) 0)
      (bind _asdefault_game_state_2 (Utilities|Casting|CastToDefaultGameState _returnvalue))
      (Default|GameEnded _asdefault_game_state_2 false))))