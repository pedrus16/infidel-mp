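; WeaponBase is a weapon Blueprint for an FPS character that fires Bolt projectiles and tracks ammo.
; StartFire passes a CanFire gate on readiness and ammo, spawns a Bolt just ahead of the owner's camera along control rotation, then decrements Ammo.
; A timer set to FireRate re-arms firing, and UpdateAmmo sends the count to the player controller's HUD.
; StopFire is an empty stub.
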(event Custom|StartFire
  (Utilities|CanFire)
  (bind _aimtransform (CallFunction|GetAimTransform))
  (Game|SpawnActorfromClass "/Game/Infidel/Blueprints/Bolt.Bolt_C" _aimtransform "AlwaysSpawn" 0 0)
  (bind _result (Math|Integer|DecrementInt (Variables|Default|GetAmmo))
    (:%20%20
      (CallFunction|UpdateAmmo _result)
      (Variables|Default|SetFireReady false)
      (Utilities|Time|SetTimerbyEvent (delegate Custom|OnFireReady) (Variables|Default|GetFireRate)))))

(event Custom|UpdateAmmo
  (params (Ammo :type Integer))
  (bind _asfpscharacter (Utilities|Casting|CastToFPSCharacter (Components|GetOwner)))
  (bind _asfpsplayer_controller (Utilities|Casting|CastToFPSPlayerController (Pawn|GetController _asfpscharacter)))
  (Default|UpdateHUDAmmo _asfpsplayer_controller Ammo))

(event Custom|StopFire)

(event Custom|OnFireReady
  (Variables|Default|SetFireReady true))

(fn ConstructionScript)

(fn GetAimTransform
  (bind _asfpscharacter (Utilities|Casting|CastToFPSCharacter (Components|GetOwner)))
  (return (Math|Transform|MakeTransform (+ (* (Math|Vector|GetForwardVector (Pawn|GetControlRotation (Pawn|GetController _asfpscharacter) :!class /Script/Engine.Controller)) 5e+01) (Transformation|GetWorldLocation (Variables|/Game/Infidel/Blueprints/FPSCharacter.FPSCharacter_C|GetFPSCamera _asfpscharacter))) (Pawn|GetControlRotation (Pawn|GetController _asfpscharacter) :!class /Script/Engine.Controller))))