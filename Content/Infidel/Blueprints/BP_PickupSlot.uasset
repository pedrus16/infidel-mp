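; BP_PickupSlot is a slot actor that captures a single Pickup and holds it in place.
; When a Pickup overlaps it while no valid Item is held, the slot stores it, turns off its physics and collision, and teleports it to the slot's box.
; It then fires the ItemPlaced dispatcher.
; Placement is one-way, as end overlap does nothing and the logic to clear the Item is disconnected.
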(event EventBeginPlay)

(event Collision|EventActorBeginOverlap
  (params (OtherActor :type Actor%20Object%20Reference))
  (Utilities|IsValid (Variables|Default|GetItem)
    (:Is%20Not%20Valid
      (bind _aspickup (Utilities|Casting|CastToPickup OtherActor))
      (Variables|Default|SetItem _aspickup)
      ;[1 1 1] Items cannot be picked up again
      (Physics|SetSimulatePhysics (Variables|/Game/Infidel/Blueprints/Pickup.Pickup_C|GetBox _aspickup) false)
      (Transformation|SetWorldLocation (Variables|/Game/Infidel/Blueprints/Pickup.Pickup_C|GetBox _aspickup) (Transformation|GetWorldLocation (Variables|Default|GetBox)) false true)
      (Collision|SetActorEnableCollision _aspickup false)
      (Default|CallItemPlaced))))

(event EventTick
  (params (DeltaSeconds :type Float%20%28single-precision%29)))

(event Collision|EventActorEndOverlap
  (params (OtherActor :type Actor%20Object%20Reference)))

(fn ConstructionScript)