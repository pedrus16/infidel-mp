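; ItemSpawnController is an actor that places a single Pickup at a randomly chosen spawn point when play begins.
; On BeginPlay it rebuilds its Spawns list from attached actors that cast to ItemSpawn.
; It then spawns the Pickup at a random entry's world location, adjusting for collisions but always spawning.
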(event EventBeginPlay
  (bind _spawns (Variables|Default|GetSpawns))
  (Utilities|Array|Clear (Variables|Default|GetSpawns))
  (for _array_element (Actor|GetAttachedActors true)
    (bind _asitem_spawn (Utilities|Casting|CastToItemSpawn _array_element))
    (Utilities|Array|Add _spawns _asitem_spawn))
  (Game|SpawnActorfromClass "/Game/Infidel/Blueprints/Pickup.Pickup_C" (Math|Conversions|ToTransform(Vector) (Transformation|GetWorldLocation (Variables|/Script/Engine.Actor|GetRootComponent (Utilities|GetRandomElement _spawns)))) "AdjustIfPossibleButAlwaysSpawn" 0 0))

(event Collision|EventActorBeginOverlap
  (params (OtherActor :type Actor%20Object%20Reference)))

(event EventTick
  (params (DeltaSeconds :type Float%20%28single-precision%29)))

(fn ConstructionScript)